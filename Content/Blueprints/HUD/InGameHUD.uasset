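; InGameHUD is the in-game HUD that manages the gameplay, help and end-game widgets.
; On BeginPlay it creates all three, shows the in-game widget and sets game-only input, with the Help action toggling the help page.
; A match state change clears all widgets and, on Lost, shows the end-game widget with UI-only input.
; Inventory changes are relayed through an event dispatcher.
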(event EventMatchStateChanged
  (params (MatchState :type EShooterMatchState%20Enum :default "Warmup"))
  (bind _endgame_widget (Variables|Default|GetEndGame_Widget))
  ;[1 1 1] Comment
  (Viewport|RemoveAllWidgets)
  (switch Utilities|FlowControl|Switch|SwitchonEShooterMatchState MatchState
    (:Lost
      (UserInterface|Viewport|AddtoViewport _endgame_widget 0)
      (Input|SetInputModeUIOnly (Game|Player|GetOwningPlayerController) _endgame_widget true))))

(event EventInventoryChanged
  (params (Inventory :type Array%20of%20FPS%20Weapon%20Object%20References))
  ;[1 1 1] Comment
  (Default|CallDispatchInventoryChanged Inventory))

(event EventBeginPlay
  (bind _returnvalue (Game|Player|GetOwningPlayerController))
  ;[1 1 1] SETUP
  (Utilities|FlowControl|Sequence
    (:then_0
      (bind _returnvalue_2 (UserInterface|CreateWidget "/Game/UMG/InGame_Widget.InGame_Widget_C"))
      (bind _output_get (Variables|Default|SetInGame_Widget _returnvalue_2))
      (UserInterface|Viewport|AddtoViewport _output_get 0))
    (:then_1
      (bind _returnvalue_3 (UserInterface|CreateWidget "/Game/UMG/EndGame_Widget.EndGame_Widget_C"))
      (Variables|Default|SetEndGame_Widget _returnvalue_3))
    (:then_2
      (bind _returnvalue_4 (UserInterface|CreateWidget "/Game/UMG/Help_Widget.Help_Widget_C"))
      (Variables|Default|SetHelp_Widget _returnvalue_4))
    (:then_3
      (Input|EnableInput _returnvalue)
      (Input|SetInputModeGameOnly _returnvalue))))

(event Input|ActionEvents|InputActionHelp
  (params (Key :type Key%20Structure :default "AnyKey"))
  (bind _help_widget (Variables|Default|GetHelp_Widget))
  ;[1 1 1] 帮助页
  (:Pressed
    (if (UserInterface|Viewport|IsinViewport _help_widget)
      (Widget|RemovefromParent _help_widget)
      (else
        (UserInterface|Viewport|AddtoViewport _help_widget 0)))))

(fn ConstructionScript)