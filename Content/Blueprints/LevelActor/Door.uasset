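; Usable door actor that swings open 90 degrees in either direction when the IUse event fires.
; A location delta rotated by actor rotation picks the swing side, meant to follow the pawn's side.
; The OpenAnim timeline blends the Door component's relative rotation toward that yaw after stopping CloseAnim.
; A CloseAnim closing blend exists but is disconnected, and the Box end-overlap event is empty.
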(event OnComponentEndOverlap(Box)
  (params (OtherActor :type Actor%20Object%20Reference) (OtherComp :type Primitive%20Component%20Object%20Reference) (OtherBodyIndex :type Integer)))

(event EventIUse
  (bind _door (Variables|Components|GetDoor))
  (Audio|Components|Audio|Stop (Variables|Default|GetCloseAnim)) ; Interrupt closing animation
  (Variables|Default|SetOpenDirection (> (.X (Math|Vector|BreakVector (Math|Vector|RotateVector (- (Transformation|GetActorLocation) (Transformation|GetActorLocation)) (Transformation|GetActorRotation)))) 0.0))
  (bind _rotation (Timeline|OpenAnim PlayFromStart)
    (:Update
      (Transformation|SetRelativeRotation _door (Math|Rotator|Lerp(Rotator) (Variables|/Script/Engine.SceneComponent|GetRelativeRotation _door) (Math|Rotator|MakeRotator 0.0 0.0 (Math|Float|SelectFloat 9e+01 -9e+01 (Variables|Default|GetOpenDirection))) _rotation true) false false))))

(fn ConstructionScript)