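; TestRoom is a room actor with gate components for snapping to other rooms, apparently for modular level assembly.
; Construction gathers its RoomGateComponents into Gates.
; GetValidGateRand adds unconnected gates to ValidGates, which is never cleared here, and returns a random entry.
; ConnectionGate repositions and rotates this room using both gates' relative transforms, resets scale to one, then marks both gates connected.
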(event EventBeginPlay)

(event EventActorBeginOverlap
  (params (OtherActor :type Actor%20Object%20Reference)))

(event EventTick
  (params (DeltaSeconds :type Float%20%28single-precision%29)))

(fn ConstructionScript
  (Utilities|Array|AppendArray (Variables|Default|GetGates) (Actor|GetComponentsByClass "/Script/FPSGame.RoomGateComponent")))

(fn GetValidGateRand
  (Utilities|FlowControl|Sequence
    (:then_0
      ;[1 1 1] 过滤
      (for _array_element (Variables|Default|GetGates)
        (if (not (Variables|/Script/FPSGame.RoomGateComponent|GetbHaveConnection _array_element))
          (Utilities|Array|AddUnique (LocalVariables|GetValidGates) _array_element))))
    (:then_1
      (if (> (Utilities|Array|Length (LocalVariables|GetValidGates)) 0)
        (return (Utilities|Array|Get(acopy) (LocalVariables|GetValidGates) (Math|Random|RandomInteger (Utilities|Array|Length (LocalVariables|GetValidGates)))))
        (else
          (return 0))))))

(fn ConnectionGate
  (params (OtherGate :type Room%20Gate%20Component%20Object%20Reference) (SelfGate :type Room%20Gate%20Component%20Object%20Reference))
  (bind _returnvalue (Transformation|GetRelativeTransform SelfGate))
  (bind (_location _rotation) (Math|Transform|BreakTransform _returnvalue))
  (Transformation|SetActorTransform (Math|Transform|MakeTransform (+ (+ (Transformation|GetActorLocation) (Variables|/Script/Engine.SceneComponent|GetRelativeLocation OtherGate)) (Variables|/Script/Engine.SceneComponent|GetRelativeLocation SelfGate)) (Variables|/Script/Engine.SceneComponent|GetRelativeRotation SelfGate)))
  (Transformation|SetActorLocation (+ (Transformation|GetActorLocation) (Math|Vector|UnrotateVector _location _rotation)) false false)
  (Variables|/Script/FPSGame.RoomGateComponent|SetbHaveConnection OtherGate true)
  (Variables|/Script/FPSGame.RoomGateComponent|SetbHaveConnection SelfGate true))