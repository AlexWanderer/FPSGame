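; VR pawn that gives the player a weapon on the left motion controller.
; On BeginPlay it spawns an actor of the class held in NewVar0, stores it as Weapon and attaches it to MotionControllerLeft.
; The left trigger starts and stops weapon fire, with the L key wired to the same calls.
; The right trigger only prints a debug string.
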(event EventBeginPlay
  (bind _returnvalue (Game|SpawnActorfromClass (Variables|Default|GetNewVar_0) (Transformation|GetActorTransform) "Undefined" 0 0))
  (bind _output_get (Variables|Default|SetWeapon _returnvalue))
  (Class|Actor|AttachRootComponentto _output_get (Variables|Default|GetMotionController_Left) "None" "KeepRelativeOffset" true))

(event EventActorBeginOverlap
  (params (OtherActor :type Actor%20Object%20Reference)))

(event EventTick
  (params (DeltaSeconds :type Float%20%28single-precision%29)))

(event Input|KeyboardEvents|MotionControllerLeftTrigger
  (params (Key :type Key%20Structure :default "AnyKey"))
  (bind _weapon (Variables|Default|GetWeapon))
  (:Pressed
    (Class|FPSWeapon|StartFire _weapon))
  (:Released
    (Class|FPSWeapon|StopFire _weapon)))

(event Input|KeyboardEvents|MotionControllerRightTrigger
  (params (Key :type Key%20Structure :default "AnyKey"))
  (:Pressed
    (Development|PrintString "Hello HTC R")))

(event Input|KeyboardEvents|L
  (params (Key :type Key%20Structure :default "AnyKey"))
  (bind _weapon (Variables|Default|GetWeapon))
  (:Pressed
    (Class|FPSWeapon|StartFire _weapon))
  (:Released
    (Class|FPSWeapon|StopFire _weapon)))

(fn ConstructionScript)